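; BP_Enemy is an AI enemy that detects the player by sight and can look around.
; PawnSensing marks the player visible unless invisible, and a retriggerable delay clears that flag shortly after sightings stop.
; Behavior Tree-triggered looking around uses a timeline to swing yaw about the starting rotation, scaled by an amplitude.
; A separate event stops that rotation when the player is found.
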(event OnSeePawn(PawnSensing)
  (params (Pawn :type Pawn%20Object%20Reference))
  ;[1 1 1] Check if the player is seen
  (Variables|Default|SetSeenPlayer Pawn)
  (bind _asbp_player (Utilities|Casting|CastToBP_Player Pawn))
  (if (not (Variables|/Game/AI_References/Assets/Blueprints/BP_Player.BP_Player_C|GetisInvisible _asbp_player))
    (Utilities|FlowControl|Sequence
      (:then_0
        (Variables|Default|SetIsPlayerVisible true))
      (:then_1
        ;;[1 1 1] Reset visibility to update if the enemy lost sight of the player
        (Utilities|FlowControl|RetriggerableDelay 0.4)
        (Variables|Default|SetIsPlayerVisible false)))))

(event Custom|StartLookingAround
  (bind _returnvalue (Transformation|GetActorRotation))
  ;[1 1 1] Rotation movement when looking around (activated from the Behaviour Tree)
  (Variables|Default|SetOriginalRotation (.yaw _returnvalue))
  (bind _rotation (Timeline|Rotation PlayFromStart)
    (:Update
      (Transformation|SetActorRotation (Math|Rotator|MakeRotator (.roll _returnvalue) (.pitch _returnvalue) (+ (* _rotation (Variables|Default|GetAmplitude)) (Variables|Default|GetOriginalRotation)))))))

(event Custom|AbortRotation
  (bind _returnvalue (Transformation|GetActorRotation))
  ;[1 1 1] Abort rotation if the enemy finds the player while looking around
  ;[1 1 1] Rotation movement when looking around (activated from the Behaviour Tree)
  (bind _rotation (Timeline|Rotation Stop)
    (:Update
      (Transformation|SetActorRotation (Math|Rotator|MakeRotator (.roll _returnvalue) (.pitch _returnvalue) (+ (* _rotation (Variables|Default|GetAmplitude)) (Variables|Default|GetOriginalRotation)))))))

(fn ConstructionScript)