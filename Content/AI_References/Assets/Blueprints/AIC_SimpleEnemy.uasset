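; AI controller for a simple enemy that starts its assigned behavior tree when play begins.
; Before running the tree, it initializes the assigned blackboard with the controlled pawn's starting location as home, its original yaw, and a zeroed target location.
; All further decision-making is left to the behavior tree, which can read these stored values.
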(event Custom|SetOriginalValues
  (bind _returnvalue (Pawn|GetControlledPawn))
  ;[1 1 1] Stores original position and z rotation in Blackboard
  (bind _blackboardcomponent (Class|AIController|UseBlackboard (Variables|Default|GetUsedBlackboard)))
  (AI|Components|Blackboard|SetValueasVector _blackboardcomponent (Variables|Default|GetHomeLocation) (Transformation|GetActorLocation _returnvalue))
  (AI|Components|Blackboard|SetValueasFloat _blackboardcomponent (Variables|Default|GetOriginalZRotation) (.yaw (Transformation|GetActorRotation _returnvalue)))
  (AI|Components|Blackboard|SetValueasVector _blackboardcomponent (Variables|Default|GetTargetLocation) "0, 0, 0"))

(event EventBeginPlay
  (CallFunction|SetOriginalValues)
  (AI|RunBehaviorTree (Variables|Default|GetUsedBehaviourTree)))

(fn ConstructionScript)